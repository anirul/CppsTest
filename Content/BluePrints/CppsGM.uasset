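; CppsGM is a game mode that gives each player who logs in a CppsPlayerPawn at a player start.
; BeginPlay caches all PlayerStart actors, and PostLogin passes the new controller to Respawn.
; Respawn destroys any existing pawn, spawns and possesses a new one at the start indexed by PlayerCount, then increments that count.
; The count rises on every respawn, with no wrap or bounds check.
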(event `self.ReceiveBeginPlay`
  (bind _outactors (`GameplayStatics.GetAllActorsOfClass` "/Script/Engine.PlayerStart"))
  (set `self.PlayerStarts` _outactors))

(event `self.K2_PostLogin`
  (params (NewPlayer :type "PlayerController Object Reference"))
  (`self.Respawn` NewPlayer))

(event `Respawn`
  (params (PlayerController :type "PlayerController Object Reference"))
  (bind _returnvalue (`Controller.K2_GetPawn` PlayerController))
  (`/Engine/EditorBlueprintResources/StandardMacros.IsValid` _returnvalue
    (:`Is Valid`
      (`self.K2_DestroyActor` _returnvalue))
    (:`Is Not Valid`
      _))
  (bind _returnvalue_2 (`|SpawnActorFromClass` "/Game/BluePrints/CppsPlayerPawn.CppsPlayerPawn_C" (`self.GetTransform` (`KismetArrayLibrary.Array_Get` (`self.PlayerStarts`) (`self.PlayerCount`))) "Undefined" "OverrideRootScale"))
  (`Controller.Possess` PlayerController _returnvalue_2)
  (set `self.PlayerCount` (+ (`self.PlayerCount`) 1)))

(fn `UserConstructionScript`)